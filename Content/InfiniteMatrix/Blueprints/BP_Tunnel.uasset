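; BP_Tunnel is an endless-tunnel segment with a rotating obstacle wall, spawning a health pickup and an enemy at random offsets on BeginPlay.
; Crossing the trigger makes TunnelSpawner add the next segment, destroys this one and awards the player a point.
; Hitting the wall damages the player, then triggers restart or a score penalty with red flash; projectiles leaving it are destroyed.
; RandomizeWall picks a hole mesh and random roll, but is not called here.
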(event `self.ReceiveTick`
  (params (DeltaSeconds :type "Float (single-precision)"))
  (`SceneComponent.K2_AddLocalRotation` (`self.WallMesh`) (`KismetMathLibrary.MakeRotator` (* DeltaSeconds (`self.RotateSpeed`))) false false))

(event `self.TriggerZone.OnComponentBeginOverlap`
  (params (OverlappedComponent :type "PrimitiveComponent Object Reference") (OtherActor :type "Actor Object Reference") (OtherComp :type "PrimitiveComponent Object Reference") (OtherBodyIndex :type Integer) (bFromSweep :type Boolean) (SweepResult :type "HitResult Structure (by ref)"))
  (bind _asbp_player (cast `/Game/InfiniteMatrix/Blueprints/BP_Player` OtherActor))
  (`/Game/InfiniteMatrix/Blueprints/BP_TunnelSpawner.Spawn Tunnel at Spawn Point` (`self.TunnelSpawner`))
  (`self.K2_DestroyActor`)
  (set `/Game/InfiniteMatrix/Blueprints/BP_Player.Player_Score` (+ (`/Game/InfiniteMatrix/Blueprints/BP_Player.Player_Score` _asbp_player) 1.0) _asbp_player))

(event `self.ReceiveBeginPlay`
  (bind _returnvalue (`KismetMathLibrary.RandomIntegerInRange` -300 300))
  (bind _returnvalue_2 (`KismetMathLibrary.RandomIntegerInRange` -300 300))
  (bind (_returnvalue_x _returnvalue_y _returnvalue_z) (`KismetMathLibrary.BreakVector` (`SceneComponent.K2_GetComponentLocation` (`self.WallMesh`))))
  (bind (_returnvalue_x_2 _returnvalue_y_2 _returnvalue_z_2) (`KismetMathLibrary.BreakVector` (`SceneComponent.K2_GetComponentLocation` (`self.WallMesh`))))
  (`|SpawnActorFromClass` "/Game/InfiniteMatrix/Blueprints/HealthPickup.HealthPickup_C" (`KismetMathLibrary.MakeTransform` (`KismetMathLibrary.MakeVector` (+ _returnvalue_x (`KismetMathLibrary.RandomIntegerInRange` 0 4000)) (+ _returnvalue_z _returnvalue_2) (+ _returnvalue_y _returnvalue_2))) "Undefined" "MultiplyWithRoot" null null)
  (`|SpawnActorFromClass` "/Game/InfiniteMatrix/Blueprints/Enemy.Enemy_C" (`KismetMathLibrary.MakeTransform` (`KismetMathLibrary.MakeVector` (+ _returnvalue_x_2 (`KismetMathLibrary.RandomIntegerInRange` 0 4000)) (+ _returnvalue_z_2 _returnvalue) (+ _returnvalue_y_2 _returnvalue))) "Undefined" "MultiplyWithRoot" null null))

(event `self.WallMesh.OnComponentBeginOverlap`
  (params (OverlappedComponent :type "PrimitiveComponent Object Reference") (OtherActor :type "Actor Object Reference") (OtherComp :type "PrimitiveComponent Object Reference") (OtherBodyIndex :type Integer) (bFromSweep :type Boolean) (SweepResult :type "HitResult Structure (by ref)"))
  (bind _asbp_player (cast `/Game/InfiniteMatrix/Blueprints/BP_Player` OtherActor))
  (bind _output_get (set `/Game/InfiniteMatrix/Blueprints/BP_Player.Health Variable` (`KismetMathLibrary.FClamp` (- (`/Game/InfiniteMatrix/Blueprints/BP_Player.Health Variable` _asbp_player) 10.0) 0.0 100.0) _asbp_player))
  (`KismetSystemLibrary.PrintString` (`KismetStringLibrary.Conv_DoubleToString` _output_get))
  (if (<= (`/Game/InfiniteMatrix/Blueprints/BP_Player.Health Variable` _asbp_player) 0.0)
    (set `/Game/InfiniteMatrix/Blueprints/BP_Player.IsDead` true _asbp_player)
    (`/Game/InfiniteMatrix/Blueprints/BP_Player.DisplayRestart` _asbp_player)
    (else
      (set `/Game/InfiniteMatrix/Blueprints/BP_Player.Player_Score` (- (`/Game/InfiniteMatrix/Blueprints/BP_Player.Player_Score` _asbp_player) 1.0) _asbp_player)
      (bind _returnvalue (`|CreateWidget` "/Game/InfiniteMatrix/Blueprints/RedFlash.RedFlash_C"))
      (`UserWidget.AddToViewport` _returnvalue 0))))

(event `self.WallMesh.OnComponentEndOverlap`
  (params (OverlappedComponent :type "PrimitiveComponent Object Reference") (OtherActor :type "Actor Object Reference") (OtherComp :type "PrimitiveComponent Object Reference") (OtherBodyIndex :type Integer))
  (bind _asprojectile (cast `/Game/InfiniteMatrix/Blueprints/projectile` OtherActor))
  (`self.K2_DestroyActor` _asprojectile))

(fn `RandomizeWall`
  (`StaticMeshComponent.SetStaticMesh` (`self.WallMesh`) (select `int` (`KismetMathLibrary.RandomIntegerInRange` 0 3) :`0` "/Game/InfiniteMatrix/Meshes/SM_Hole_01.SM_Hole_01" :`1` "/Game/InfiniteMatrix/Meshes/SM_Hole_02.SM_Hole_02" :`2` "/Game/InfiniteMatrix/Meshes/SM_Hole_03.SM_Hole_03" :`3` "/Game/InfiniteMatrix/Meshes/SM_Hole_04.SM_Hole_04" :!type "StaticMesh Object Reference"))
  (`SceneComponent.K2_AddLocalRotation` (`self.WallMesh`) (`KismetMathLibrary.MakeRotator` (`KismetMathLibrary.RandomFloatInRange` 0.0 360.0)) false false))

(fn `UserConstructionScript`)